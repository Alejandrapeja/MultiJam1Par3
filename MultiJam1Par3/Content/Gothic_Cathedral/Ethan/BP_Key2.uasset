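; BP_Key2 is a pickup key actor that shows a prompt widget when the player is nearby.
; A sphere overlap checks for the Player tag and toggles the widget's visibility on enter and exit.
; The PickUp_Key2 event, not called within this Blueprint, destroys the actor and plays a 2D key sound.
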(event `PickUp_Key2`
  (`self.K2_DestroyActor`)
  (`GameplayStatics.PlaySound2D` "/Game/Gothic_Cathedral/Ethan/Key.Key" 1.0 1.0 0.0 null null))

(event `self.Sphere.OnComponentBeginOverlap`
  (params (OverlappedComponent :type "PrimitiveComponent Object Reference") (OtherActor :type "Actor Object Reference") (OtherComp :type "PrimitiveComponent Object Reference") (OtherBodyIndex :type Integer) (bFromSweep :type Boolean) (SweepResult :type "HitResult Structure (by ref)"))
  (if (`self.ActorHasTag` OtherActor "Player")
    (`SceneComponent.SetVisibility` (`self.Widget`) true false)))

(event `self.Sphere.OnComponentEndOverlap`
  (params (OverlappedComponent :type "PrimitiveComponent Object Reference") (OtherActor :type "Actor Object Reference") (OtherComp :type "PrimitiveComponent Object Reference") (OtherBodyIndex :type Integer))
  (if (`self.ActorHasTag` OtherActor "Player")
    (`SceneComponent.SetVisibility` (`self.Widget`) false false)))

(fn `UserConstructionScript`)