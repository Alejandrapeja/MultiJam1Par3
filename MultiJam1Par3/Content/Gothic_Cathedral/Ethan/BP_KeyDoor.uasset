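; BP_KeyDoor is a double door that swings open and closed when its PuertaLLave ("key door") event is called.
; A timeline drives the yaw of two meshes, Cube and Cube1, from 0 to 90 degrees in opposite directions.
; IsClose selects playing from start or reversing, and flips each time the timeline finishes.
; The Blueprint itself contains no key check.
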(event `PuertaLLave`
  (if (`self.IsClose`)
    (bind (_direction _newtrack_0) (`Timeline|Timeline_1` :!via `PlayFromStart` :!label _label)
      (:`Update`
        (`SceneComponent.K2_SetRelativeRotation` (`self.Cube`) (`KismetMathLibrary.MakeRotator` 0.0 0.0 (`KismetMathLibrary.Lerp` 0.0 90.0 _newtrack_0)) false false)
        (`SceneComponent.K2_SetRelativeRotation` (`self.Cube1`) (`KismetMathLibrary.MakeRotator` 0.0 0.0 (`KismetMathLibrary.Lerp` 0.0 -90.0 _newtrack_0)) false false))
      (:`Finished`
        (set `self.IsClose` (not (`self.IsClose`)))))
    (else
      (goto _label :!via `Reverse`))))

(fn `UserConstructionScript`)