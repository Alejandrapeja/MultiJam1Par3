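; BP_KeyDoor1 is a double door that swings open or closed when its PuertaLLave2 event is called.
; A timeline rotates two cube leaves in opposite directions, playing or reversing according to IsClose, which flips when it finishes.
; The wooden door sound is triggered on every timeline update, not once per swing.
; A box trigger shows a widget while a Player-tagged actor overlaps it; no key check happens here.
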(event `PuertaLLave2`
  (if (`self.IsClose`)
    (bind (_direction _newtrack_0) (`Timeline|Timeline_1` :!via `PlayFromStart` :!label _label)
      (:`Update`
        (`SceneComponent.K2_SetRelativeRotation` (`self.Cube`) (`KismetMathLibrary.MakeRotator` 0.0 0.0 (`KismetMathLibrary.Lerp` 0.0 90.0 _newtrack_0)) false false)
        (`SceneComponent.K2_SetRelativeRotation` (`self.Cube1`) (`KismetMathLibrary.MakeRotator` 0.0 0.0 (`KismetMathLibrary.Lerp` 0.0 -90.0 _newtrack_0)) false false)
        (`GameplayStatics.PlaySound2D` "/Game/Gothic_Cathedral/Ethan/WoodenDoor.WoodenDoor" 0.2 1.0 0.0 null null))
      (:`Finished`
        (set `self.IsClose` (not (`self.IsClose`)))))
    (else
      (goto _label :!via `Reverse`))))

(event `self.Box.OnComponentBeginOverlap`
  (params (OverlappedComponent :type "PrimitiveComponent Object Reference") (OtherActor :type "Actor Object Reference") (OtherComp :type "PrimitiveComponent Object Reference") (OtherBodyIndex :type Integer) (bFromSweep :type Boolean) (SweepResult :type "HitResult Structure (by ref)"))
  (if (`self.ActorHasTag` OtherActor "Player")
    (`SceneComponent.SetVisibility` (`self.Widget`) true false)))

(event `self.Box.OnComponentEndOverlap`
  (params (OverlappedComponent :type "PrimitiveComponent Object Reference") (OtherActor :type "Actor Object Reference") (OtherComp :type "PrimitiveComponent Object Reference") (OtherBodyIndex :type Integer))
  (if (`self.ActorHasTag` OtherActor "Player")
    (`SceneComponent.SetVisibility` (`self.Widget`) false false)))

(fn `UserConstructionScript`)