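; BP_Enemy_Ciego is an enemy (Ciego, "blind") that investigates where it perceives the player character.
; A successful AI Perception stimulus from BP_ThirdPersonCharacter1MARCO sends it to the stimulus location via AI MoveTo.
; An Investigation flag ignores new stimuli until one second after a successful move, and is never reset on failure.
; An unconnected loop that would periodically relocate it randomly around the player never runs.
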(event `self.AIPerception.OnTargetPerceptionUpdated`
  (params (Actor :type "Actor Object Reference") (Stimulus :type "AIStimulus Structure"))
  (bind (_age _expirationage _strength _stimuluslocation _receiverlocation _tag _bsuccessfullysensed) (break `AIStimulus` Stimulus))
  (cast `/Game/ThirdPerson/Blueprints/BP_ThirdPersonCharacter1MARCO` Actor)
  (if _bsuccessfullysensed
    (if (not (`self.Investigation`))
      (set `self.Investigation` true)
      (`|AIMoveTo` self _stimuluslocation null
        (:`OnSuccess`
          (`KismetSystemLibrary.Delay` 1.0)
          (set `self.Investigation` false))))))

(event `self.ReceiveBeginPlay`)

(fn `UserConstructionScript`)