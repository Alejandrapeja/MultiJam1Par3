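; Enemy statue that chases player 0 only while the player is not looking at it.
; Each tick it either stops active movement or issues AI MoveTo toward the player, based on the IsPlayerSee flag.
; The CanMove event sets that flag from outside.
; A random teleport loop, offsetting X and Y every ten seconds, is left disconnected from BeginPlay and never runs.
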(event `self.ReceiveTick`
  (params (DeltaSeconds :type "Float (single-precision)"))
  ;[1 1 1] Si no lo esta mirando
  (if (`self.isPlayerSee`)
    (`NavMovementComponent.StopActiveMovement` (`self.CharacterMovement`))
    (else
      (`|AIMoveTo` self (0.0 0.0 0.0) (`GameplayStatics.GetPlayerCharacter` 0)))))

(event `self.CanMove`
  (params (seePlayer :type Boolean))
  ;[1 1 1] Puede moverse
  (set `self.isPlayerSee` seePlayer))

(event `self.ReceiveBeginPlay`
  ;[1 1 1] Tp Aleatorio
)

(fn `UserConstructionScript`)