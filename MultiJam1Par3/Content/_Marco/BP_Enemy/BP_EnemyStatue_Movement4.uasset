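; Enemy statue that chases the player while unseen and freezes while watched.
; Tick stops active movement when IsPlayerSee is set, otherwise reissues AIMoveTo toward the player character every frame.
; The CanMove event sets that flag from its SeePlayer input, with no sight detection in this Blueprint.
; A BeginPlay delay loop periodically teleports the statue by a random X/Y offset, whether seen or not.
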(event `self.ReceiveTick`
  (params (DeltaSeconds :type "Float (single-precision)"))
  ;[1 1 1] Si no lo esta mirando
  (if (`self.isPlayerSee`)
    (`NavMovementComponent.StopActiveMovement` (`self.CharacterMovement`))
    (else
      (`|AIMoveTo` self (0.0 0.0 0.0) (`GameplayStatics.GetPlayerCharacter` 0)))))

(event `self.CanMove`
  (params (seePlayer :type Boolean))
  ;[1 1 1] Puede moverse
  (set `self.isPlayerSee` seePlayer))

(event `self.ReceiveBeginPlay`
  (bind (_returnvalue_x _returnvalue_y) (`KismetMathLibrary.BreakVector` (`self.K2_GetActorLocation`)))
  ;[1 1 1] Tp Aleatorio
  (`KismetSystemLibrary.Delay` 10.0 :!label _label)
  (`self.K2_SetActorRelativeLocation` (`KismetMathLibrary.MakeVector` (+ _returnvalue_x (`KismetMathLibrary.RandomFloatInRange` -500.0 500.0)) (+ _returnvalue_y (`KismetMathLibrary.RandomFloatInRange` -500.0 500.0))))
  (goto _label))

(fn `UserConstructionScript`)